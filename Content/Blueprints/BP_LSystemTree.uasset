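; Actor that generates a branching L-system tree from an axiom and X/F rewrite rules, on construction and at BeginPlay.
; StartLSystem runs Evolve over several generations to expand the sentence, then prints it and sends it to a widget.
; GenerateTree walks the sentence turtle-style with a Sphere component, moving on F and yawing on +/-.
; Brackets open and close branches stored with parent indices; F steps are visualized only as temporary debug spheres.
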(event EventBeginPlay
  (CallFunction|StartLSystem)
  (CallFunction|GenerateTree))

(event Collision|EventActorBeginOverlap
  (params (OtherActor :type Actor%20Object%20Reference)))

(event EventTick
  (params (DeltaSeconds :type Float%20%28single-precision%29)))

(fn ConstructionScript
  (CallFunction|StartLSystem)
  (CallFunction|GenerateTree))

(fn Evolve
  (bind _output_get (LocalVariables|SetLocal_CurrentSentence (Utilities|String|GetCharacterArrayfromString (Variables|Default|GetCurrentSentence))))
  (for _array_element _output_get
    (switch string _array_element
      (:X
        ;[0 0.1809 1] If Char is X
        (Variables|Default|SetNextSentence (Utilities|String|Append (Variables|Default|GetNextSentence) (Variables|Default|GetXRule))))
      (:F
        ;[0 0.1809 1] If Char is F
        (Variables|Default|SetNextSentence (Utilities|String|Append (Variables|Default|GetNextSentence) (Variables|Default|GetFRule))))
      (:+
        ;[0 0.1809 1] Not A Rule
        (Variables|Default|SetNextSentence (Utilities|String|Append (Variables|Default|GetNextSentence) _array_element) :!label _label))
      (:-
        (goto _label))
      (:[
        (goto _label))
      (:]
        (goto _label))))
  (Variables|Default|SetCurrentSentence (Variables|Default|GetNextSentence))
  (Variables|Default|SetNextSentence ""))

(fn StartLSystem
  (params (WidgetRef :type WBP%20Testing%20Object%20Reference))
  (Variables|Default|SetCurrentSentence (Variables|Default|GetAxiom))
  (Variables|Default|SetNextSentence "")
  (for _index (range 0 (Variables|Default|GetGenerations))
    (CallFunction|Evolve))
  (Default|UpdateText WidgetRef (Utilities|Text|ToText(String) (Variables|Default|GetCurrentSentence)))
  (Development|PrintString (Variables|Default|GetCurrentSentence)))

(fn GenerateTree
  (bind _sphere (Variables|Default|GetSphere))
  (bind _sphere_2 (Variables|Default|GetSphere))
  (Variables|Default|SetCurrentBranchIndex 0)
  (Variables|Default|SetTree (Utilities|Array|MakeArray (Utilities|Struct|MakeBranch (Utilities|Array|MakeArray (Transformation|GetRelativeTransform (Variables|Default|GetSphere))) -1)))
  (bind _output_get (LocalVariables|SetLocalCurrent (Utilities|String|GetCharacterArrayfromString (Variables|Default|GetCurrentSentence))))
  (for _index (range 0 (- (Utilities|Array|Length _output_get) 1))
    (switch string (Utilities|Array|Get(acopy) (LocalVariables|GetLocalCurrent) _index)
      (:F
        ;[1 1 1] Move Forward
        (Transformation|AddRelativeLocation _sphere_2 (* (Math|Vector|GetForwardVector (Variables|/Script/Engine.SceneComponent|GetRelativeRotation (Variables|Default|GetSphere))) (Variables|Default|GetLength)) false false)
        (Utilities|Array|Add (.Points (Utilities|Struct|BreakBranch (Utilities|Array|Get(acopy) (Variables|Default|GetTree) (Variables|Default|GetCurrentBranchIndex)))) (Transformation|GetRelativeTransform _sphere_2))
        (Rendering|Debug|DrawDebugSphere (Transformation|GetWorldLocation (Variables|Default|GetSphere)) 5.0 12 "(R=0.058105,G=0.656250,B=0.588370,A=1.000000)" 1e+01))
      (:+
        ;[1 1 1] Rotate clockwise
        (Transformation|AddRelativeRotation _sphere (Math|Rotator|MakeRotator 0.0 0.0 (Variables|Default|GetAngle)) false false)
        (Transformation|AddLocalRotation _sphere "0, 0, 0" false false))
      (:-
        ;[1 1 1] Rotate Counterclockwise
        (Transformation|AddRelativeRotation (Variables|Default|GetSphere) (Math|Rotator|MakeRotator 0.0 0.0 (* (Variables|Default|GetAngle) -1.0)) false false))
      (:[
        ;[1 1 1] New branch
        (bind _returnvalue (Utilities|Array|Add (Variables|Default|GetTree) (Utilities|Struct|MakeBranch (Utilities|Array|MakeArray (Transformation|GetRelativeTransform (Variables|Default|GetSphere))) (Variables|Default|GetCurrentBranchIndex))))
        (Variables|Default|SetCurrentBranchIndex _returnvalue))
      (:]
        ;[1 1 1] Return to parent branch
        (Transformation|SetRelativeTransform (Variables|Default|GetSphere) (Utilities|Array|Get(acopy) (.Points (Utilities|Struct|BreakBranch (Utilities|Array|Get(acopy) (Variables|Default|GetTree) (Variables|Default|GetCurrentBranchIndex))))) false false)
        (Variables|Default|SetCurrentBranchIndex (.ParentIndex (Utilities|Struct|BreakBranch (Utilities|Array|Get(acopy) (Variables|Default|GetTree) (Variables|Default|GetCurrentBranchIndex)))))))))